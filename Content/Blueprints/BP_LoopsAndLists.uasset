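; Demo actor for loop and array techniques, reporting mostly through printed strings.
; BeginPlay starts two self-repeating delayed loops (a game loop and a resetting recursive counter), enables input, and gathers all BP_Key actors.
; ChangeKeyColor re-calls itself on a delay, recoloring each key through dynamic materials and reshuffling keys and colors when either list runs out.
; Input triggers a while loop and name-array printouts; Tick logging is disconnected.
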(event Custom|SimpleGameLoop
  (Development|PrintString "Starting Game Loop" true true "(R=0.000000,G=0.237187,B=0.846000,A=1.000000)" 0.6 :!label _label) ; Print String
  (Utilities|FlowControl|Delay 1.0) ; Wait a sec
  (goto _label))

(event Custom|Recursive%20Loop
  ;[0.2854 1 0.3652] Comment
  (if (< (Variables|Default|GetRecursion%20Counter) 5)
    (bind _result (Math|Integer|IncrementInt (Variables|Default|GetRecursion%20Counter))
      (:%20%20
        (Development|PrintString (Utilities|String|Append "The Loop has run " (Utilities|String|ToString(Integer) _result) " times.") true true "(R=1.000000,G=0.807292,B=0.917186,A=1.000000)")
        (Utilities|FlowControl|Delay 2.0)))
    (else
      (Development|PrintString "resetting counter")
      (Variables|Default|SetRecursion%20Counter 0)
      (Utilities|FlowControl|Delay 4.0)))
  (CallFunction|RecursiveLoop))

(event Custom|FirstArray%20Test
  (bind _array (Utilities|Array|MakeArray "Leia" "Luke" "Han" "Chewie" "Artoo" "Threepio"))
  (Development|PrintString (Utilities|String|Append "Our array of names has " (Utilities|String|ToString(Integer) (Utilities|Array|Length _array)) " names in it"))
  (Development|PrintString (Utilities|String|Append "The first name on the list is " (Utilities|Array|Get(acopy) _array))))

(event Custom|List%20all%20names
  (for (_array_element _array_index) (Utilities|Array|MakeArray "Leia" "Luke" "Han" "Chewie" "Artoo" "Threepio")
    (Development|PrintString (Utilities|String|Append (Utilities|String|ToString(Integer) (+ _array_index 1)) ". " _array_element) true true "(R=1.000000,G=0.227157,B=0.197308,A=1.000000)")))

(event Custom|Change%20Key%20Color
  (if (or (>= (Variables|Default|GetColor%20Key%20Index) (Utilities|Array|Length (Variables|Default|GetColors))) (>= (Variables|Default|GetColor%20Key%20Index) (Utilities|Array|Length (Variables|Default|GetKeys)))) ; if true, reshuffle all keys and colors, and reset color key index else, change color of next key
    ;[1 1 1] Shuffle/Reset
    (Utilities|Array|Shuffle (Variables|Default|GetColors))
    (Utilities|Array|Shuffle (Variables|Default|GetKeys))
    (Variables|Default|SetColor%20Key%20Index 0))
  (Utilities|IsValid (Utilities|Array|Get(acopy) (Variables|Default|GetKeys) (Variables|Default|GetColor%20Key%20Index))
    (:Is%20Valid
      ;[1 1 1] Set the color of the key handle
      (bind _returnvalue (Rendering|Material|CreateDynamicMaterialInstance (Variables|/Game/Blueprints/BP_Key.BP_Key_C|GetCylinder (Utilities|Array|Get(acopy) (Variables|Default|GetKeys) (Variables|Default|GetColor%20Key%20Index))) 0 "/Game/Materials/M_Base.M_Base" "None" :!class /Script/Engine.PrimitiveComponent))
      (Rendering|Material|SetVectorParameterValue _returnvalue "Base Color" (Math|Conversions|ToLinearColor(Color) (Utilities|Array|Get(acopy) (Variables|Default|GetColors) (Variables|Default|GetColor%20Key%20Index))) :!class /Script/Engine.MaterialInstanceDynamic)
      (Math|Integer|IncrementInt (Variables|Default|GetColor%20Key%20Index)
        (:%20%20
          _)))
    (:Is%20Not%20Valid
      (bind _outactors (Actor|GetAllActorsOfClass "/Game/Blueprints/BP_Key.BP_Key_C"))
      (Variables|Default|SetKeys _outactors)))
  (Utilities|FlowControl|Delay 0.5)
  (CallFunction|ChangeKeyColor))

(event EventBeginPlay
  (Development|PrintString "LoopsAndLists is starting")
  (Utilities|FlowControl|Sequence
    (:then_0
      ;[1 1 1] setup
      (CallFunction|SimpleGameLoop)
      (Input|EnableInput (Game|GetPlayerController 0))
      (CallFunction|RecursiveLoop))
    (:then_1
      ;[1 1 1] setup for lists
      (bind _outactors (Actor|GetAllActorsOfClass "/Game/Blueprints/BP_Key.BP_Key_C"))
      (Variables|Default|SetKeys _outactors)
      (CallFunction|ChangeKeyColor))))

(event Collision|EventActorBeginOverlap
  (params (OtherActor :type Actor%20Object%20Reference)))

(event EventTick
  (params (DeltaSeconds :type Float%20%28single-precision%29)))

(event Input|ActionEvents|InputActionStartWhileLoop
  (params (Key :type Key%20Structure :default "None"))
  (:Pressed
    (Development|PrintString "Starting While Loop")
    (while (< (Variables|Default|GetWhileLoopCounter) 25)
      ;[0.9227 0.2723 1] While Loops Body
      (Math|Integer|IncrementInt (Variables|Default|GetWhileLoopCounter)
        (:%20%20
          (Development|PrintString (Utilities|String|Append "This while loop has run " (Utilities|String|ToString(Integer) (Variables|Default|GetWhileLoopCounter)) " times.")))))
    (Development|PrintString "the while loop is complete")
    (Variables|Default|SetWhileLoopCounter 0)))

(event Input|KeyboardEvents|6
  (params (Key :type Key%20Structure :default "None"))
  (:Pressed
    (CallFunction|FirstArrayTest)))

(event Input|KeyboardEvents|5
  (params (Key :type Key%20Structure :default "None"))
  (:Pressed
    (CallFunction|ListAllNames)))

(fn ConstructionScript)