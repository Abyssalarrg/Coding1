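; BP_FallingPlatform is a platform that drops shortly after the custom third-person character enters its trigger box, then returns to its start transform.
; A Ready flag gates a delayed chain of Activate, Drop and Reset events, with a material swap and debug print marking the stages.
; Drop enables physics simulation on the cube; Reset disables it and uses a timeline to lerp location and rotation back before re-arming.
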(event OnComponentBeginOverlap(Box)
  (params (OverlappedComponent :type Primitive%20Component%20Object%20Reference) (OtherActor :type Actor%20Object%20Reference) (OtherComp :type Primitive%20Component%20Object%20Reference) (OtherBodyIndex :type Integer) (bFromSweep :type Boolean) (SweepResult :type Hit%20Result%20Structure%20%28by%20ref%29))
  (Utilities|Casting|CastToBP_ThirdPersonCharacterCustom OtherActor)
  (CallFunction|Activate))

(event Custom|Activate
  ;[0.2226 1 0.2539] Platform Activates
  (if (Variables|Default|Getready)
    (Development|PrintString "One second left")
    (Variables|Default|Setready false)
    (Rendering|Material|SetMaterial (Variables|Default|GetCube) 0 "/Game/Materials/MI_PlatformActivated.MI_PlatformActivated")
    (Utilities|FlowControl|Delay 1.0)
    (CallFunction|Drop)))

(event Custom|Reset
  ;[1 0.8481 0.1955] Platform Resets
  (Development|PrintString "resetting")
  (Variables|Default|SetResetTransform (Transformation|GetWorldTransform (Variables|Default|GetCube)))
  (Physics|SetSimulatePhysics (Variables|Default|GetCube) false)
  (Rendering|Material|SetMaterial (Variables|Default|GetCube) 0 "/Game/Materials/MI_PlatformResetting.MI_PlatformResetting")
  (bind _float (Timeline|GoBackToStart PlayFromStart)
    (:Update
      (Transformation|SetWorldLocationAndRotation (Variables|Default|GetCube) (.location (Math|Transform|Lerp(Transform) (Variables|Default|GetResetTransform) (Variables|Default|GetStartingTransform) _float)) (.rotation (Math|Transform|Lerp(Transform) (Variables|Default|GetResetTransform) (Variables|Default|GetStartingTransform) _float)) false false))
    (:Finished
      (Variables|Default|Setready true)
      (Rendering|Material|SetMaterial (Variables|Default|GetCube) 0 "/Game/Materials/MI_PlatformReady.MI_PlatformReady"))))

(event Custom|Drop
  ;[1 0.2711 0.9883] Platform Drops
  (Development|PrintString "Dropping")
  (Physics|SetSimulatePhysics (Variables|Default|GetCube) true)
  (Rendering|Material|SetMaterial (Variables|Default|GetCube) 0 "/Game/Materials/MI_PlatformFalling.MI_PlatformFalling")
  (Utilities|FlowControl|Delay 3.0)
  (CallFunction|Reset))

(event EventBeginPlay
  (Variables|Default|SetStartingTransform (Transformation|GetWorldTransform (Variables|Default|GetCube))))

(event Collision|EventActorBeginOverlap
  (params (OtherActor :type Actor%20Object%20Reference)))

(event EventTick
  (params (DeltaSeconds :type Float%20%28single-precision%29)))

(fn ConstructionScript)